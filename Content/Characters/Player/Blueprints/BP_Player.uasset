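; Player character built on the Gameplay Ability System, granting abilities and applying level and stamina-regen effects on BeginPlay.
; Attribute change events update HUD bars, spawn damage popups, toggle the armor tag and, at zero HP, fade out, load the save and reopen the level.
; Inputs trigger tag-based abilities and a pausing backpack; Interact sphere-traces for quest NPCs, pickups and boxes.
; LoadGAS restores saved attributes through a SetByCaller effect.
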(event Custom|SetPlayerState
  (params (DelayTime :type Float%20%28double-precision%29) (MaxWalkSpeed :type Float%20%28double-precision%29))
  ;[0 0 0] 设置玩家攻击时的状态
  (Variables|Default|SetCanAttack? true)
  (Variables|/Script/Engine.CharacterMovementComponent|SetMaxWalkSpeed (Variables|Character|GetCharacterMovement) MaxWalkSpeed)
  (Utilities|FlowControl|Delay DelayTime)
  (Variables|Default|SetCanAttack? false)
  (Variables|/Script/Engine.CharacterMovementComponent|SetMaxWalkSpeed (Variables|Character|GetCharacterMovement) (.ReturnValue (Ability|Attribute|GetFloatAttributefromAbilitySystemComponent (Variables|Default|GetMyASC) "(AttributeName=\"WalkSpeed\",Attribute=/Script/GAME2D.BaseAttributeSet:WalkSpeed,AttributeOwner=\"/Script/CoreUObject.Class'/Script/GAME2D.BaseAttributeSet'\")"))))

(event Custom|LoadGAS
  (params (LoadHP :type Float%20%28double-precision%29) (LoadMP :type Float%20%28double-precision%29) (LoadArmor :type Float%20%28double-precision%29))
  (bind _returnvalue (Ability|GameplayEffect|AssignTagSetbyCallerMagnitude (GameplayEffects|MakeOutgoingSpec :self (Variables|Default|GetMyASC) :GameplayEffectClass "/Game/GAS/Abilities/Player_Abilities/GE_LoadData.GE_LoadData_C") "(TagName=\"Data.Restore.HP\")" LoadHP))
  (bind _returnvalue_2 (Ability|GameplayEffect|AssignTagSetbyCallerMagnitude _returnvalue "(TagName=\"Data.Restore.MP\")" LoadMP))
  (bind _returnvalue_3 (Ability|GameplayEffect|AssignTagSetbyCallerMagnitude _returnvalue_2 "(TagName=\"Data.Restore.Armor\")" LoadArmor))
  (GameplayEffects|ApplyGameplayEffectSpecToSelf (Variables|Default|GetMyASC) _returnvalue_3))

(event Custom|CheckBPArray
  ;[0 0.04964 1] 调试板块
  ;;[0 0 0] 检查物品数组
  (for _array_element (Variables|/Script/GAME2D.MyGameInstance|GetBackPack_Array (Class|MyBlueprintFunctionLibrary|GetGameInstanceBase))
    (Development|PrintString (Utilities|String|Append (.Name (Utilities|Struct|BreakItem_Struct _array_element)) "     Count:" (Utilities|String|ToString(Integer) (.Count (Utilities|Struct|BreakItem_Struct _array_element))) "    Class:" (Utilities|GetDisplayName (.ItemClass (Utilities|Struct|BreakItem_Struct _array_element)))))))

(event Custom|PlayerAttack
  ;[1 0.3552 0.3552] 玩家技能板块（GAS）
  ;;[0 0 0] 技能1：攻击
  (switch string (Variables|Default|GetEquippingWeapon)
    (:Default
      (CallFunction|ActiveAbilitySelf :!label _label))
    (:Sword
      (goto _label))
    (:Book
      (CallFunction|ActiveAbilitySelf 3))))

(event Custom|OnEXPChange
  (bind _returnvalue (Class|MyBlueprintFunctionLibrary|GetHUDAllUI))
  ;[1 1 1] 设置经验条
  (Utilities|IsValid _returnvalue
    (:Is%20Valid
      (Progress|SetPercent (Variables|/Script/GAME2D.UMG_Main|GetBar_Experience (Variables|/Script/GAME2D.HUD_All_UI|GetUMG_Main _returnvalue)) (/ (Math|Float|%(Float) (Variables|/Script/GAME2D.MyGameInstance|GetPlayerXP (Class|MyBlueprintFunctionLibrary|GetGameInstanceBase)) 1e+02) 1e+02)))))

(event Custom|BackpackGate
  (bind _returnvalue (Class|MyBlueprintFunctionLibrary|GetPlayerController))
  ;[1 1 1] 背包开关
  (if (Variables|Default|GetIsOpenBP?)
    (bind _bp_backpack (Variables|Default|GetBP_Backpack)
      (:then
        (Widget|RemovefromParent _bp_backpack)
        (Input|SetInputModeGameOnly _returnvalue false)
        (Variables|Default|SetIsOpenBP? false)
        (Game|SetGamePaused false))
      (:else))
    (else
      (bind _returnvalue_2 (UserInterface|CreateWidget "/Game/System/BackPackSystem/Blueprints/UI/UMG_Backpack.UMG_Backpack_C"))
      (bind _output_get (Variables|Default|SetBP_Backpack _returnvalue_2))
      (UserInterface|Viewport|AddtoViewport _output_get 0)
      (Input|SetInputModeUIOnly _returnvalue 0 "DoNotLock" false)
      (Variables|Default|SetIsOpenBP? true)
      (Game|SetGamePaused true))))

(event Custom|PlayerDamagePop
  ;[0 0 0] 设置伤害跳字
  (if (!= (Variables|Default|GetCurrentHP) (Variables|Default|GetNewHP))
    (bind _returnvalue (UserInterface|CreateWidget "/Game/UMG/DamagePopout.DamagePopout_C" 0 self (- (Variables|Default|GetCurrentHP) (Variables|Default|GetNewHP))))
    (UserInterface|Viewport|AddtoViewport _returnvalue 0)
    (Variables|Default|SetCurrentHP (.ReturnValue (Ability|Attribute|GetFloatAttributefromAbilitySystemComponent (Variables|Default|GetMyASC) "(AttributeName=\"HP\",Attribute=/Script/GAME2D.BaseAttributeSet:HP,AttributeOwner=\"/Script/CoreUObject.Class'/Script/GAME2D.BaseAttributeSet'\")")))))

(event Custom|PlayerReturn
  (bind _returnvalue (UserInterface|CreateWidget "/Game/UMG/EnterAndExitMap.EnterAndExitMap_C"))
  (UserInterface|Viewport|AddtoViewport _returnvalue 0)
  (Default|PlaytoBlack _returnvalue)
  (Class|MyBlueprintFunctionLibrary|PlayerMoveController false)
  (Utilities|FlowControl|Delay 2.0)
  (Default|EventLoadGame (.BP_Player%20Controller (CallFunction|GetPlayerandPC)))
  (Game|OpenLevel(byName) (Variables|/Script/GAME2D.MyGameInstance|GetCurrentMapName (Class|MyBlueprintFunctionLibrary|GetGameInstanceBase))))

(event Input|EnhancedActionEvents|EnhancedInputActionIA_Sword_Attack
  (params (ActionValue :type Boolean) (ElapsedSeconds :type Float%20%28double-precision%29) (TriggeredSeconds :type Float%20%28double-precision%29) (InputAction :type Input%20Action%20Object%20Reference :default "/Game/Characters/Player/Input/Actions/IA_Sword_Attack.IA_Sword_Attack"))
  ;[1 0.3552 0.3552] 玩家技能板块（GAS）
  ;;[0 0 0] 技能1：攻击
)

(event Input|EnhancedActionEvents|EnhancedInputActionIA_Dash
  (params (ActionValue :type Boolean) (ElapsedSeconds :type Float%20%28double-precision%29) (TriggeredSeconds :type Float%20%28double-precision%29) (InputAction :type Input%20Action%20Object%20Reference :default "/Game/Characters/Player/Input/Actions/IA_Dash.IA_Dash"))
  ;[1 0.3552 0.3552] 玩家技能板块（GAS）
  ;;[0 0 0] 技能3：冲刺
  (CallFunction|ActiveAbilitySelf 2))

(event Input|EnhancedActionEvents|EnhancedInputActionIA_SwordChi
  (params (ActionValue :type Boolean) (ElapsedSeconds :type Float%20%28double-precision%29) (TriggeredSeconds :type Float%20%28double-precision%29) (InputAction :type Input%20Action%20Object%20Reference :default "/Game/Characters/Player/Input/Actions/IA_SwordChi.IA_SwordChi"))
  ;[1 0.3552 0.3552] 玩家技能板块（GAS）
  ;;[0 0 0] 技能2：剑气
  (if (Utilities|Enum|Equal(Enum) (Variables|Default|GetEquippingWeapon) "Sword")
    (CallFunction|ActiveAbilitySelf 1)))

(event Input|EnhancedActionEvents|EnhancedInputActionIA_OpenBP
  (params (ActionValue :type Boolean) (ElapsedSeconds :type Float%20%28double-precision%29) (TriggeredSeconds :type Float%20%28double-precision%29) (InputAction :type Input%20Action%20Object%20Reference :default "/Game/Characters/Player/Input/Actions/IA_OpenBP.IA_OpenBP"))
  ;[1 1 1] 背包开关
  (CallFunction|BackpackGate))

(event EventBeginPlay
  (|CallParentFunction)
  (Utilities|FlowControl|Sequence
    (:then_0
      (Utilities|FlowControl|Delay 2.0)
      (Class|TaskSystemComp|SetTaskTipandTarget (Variables|Default|GetTaskSystemComp))
      (GameplayEffects|ApplyGameplayEffectToSelf :self (Variables|Default|GetMyASC) :GameplayEffectClass "/Game/GAS/Abilities/Player_Abilities/GE_LevelUp.GE_LevelUp_C" :Level (Math|Conversions|ToFloat(Integer) (Variables|/Script/GAME2D.MyGameInstance|GetPlayerLevel (Class|MyBlueprintFunctionLibrary|GetGameInstanceBase))))
      (CallFunction|OnEXPChange))
    (:then_1
      (for _array_element (Variables|Default|GetAllAbilityClass)
        (GameplayAbilities|GiveAbility (Variables|Default|GetMyASC) _array_element 0 -1)))
    (:then_2
      ;[1 1 1] 挂一个持续恢复体力的效果
      (GameplayEffects|ApplyGameplayEffectToSelf :self (Variables|Default|GetMyASC) :GameplayEffectClass "/Game/GAS/Abilities/Player_Abilities/GE_RestoreEnergy.GE_RestoreEnergy_C"))))

(event EventStrengthChangeEvent事件
  (params (NewVal :type Float%20%28single-precision%29))
  (bind _returnvalue (Class|MyBlueprintFunctionLibrary|GetHUDAllUI))
  ;[1 0.8622 0 0] 设置体力条
  (Utilities|IsValid _returnvalue
    (:Is%20Valid
      (Progress|SetPercent (Variables|/Script/GAME2D.UMG_Main|GetBar_Strength (Variables|/Script/GAME2D.HUD_All_UI|GetUMG_Main _returnvalue)) (/ NewVal (.ReturnValue (Ability|Attribute|GetFloatAttributefromAbilitySystemComponent (Variables|Default|GetMyASC) "(AttributeName=\"MAX_Strength\",Attribute=/Script/GAME2D.BaseAttributeSet:MAX_Strength,AttributeOwner=\"/Script/CoreUObject.Class'/Script/GAME2D.BaseAttributeSet'\")")))))))

(event EventMPChangeEvent事件
  (params (NewVal :type Float%20%28single-precision%29))
  (bind _returnvalue (Class|MyBlueprintFunctionLibrary|GetHUDAllUI))
  ;[0 0.07722 1 0] 设置蓝条
  (Utilities|IsValid _returnvalue
    (:Is%20Valid
      (Progress|SetPercent (Variables|/Script/GAME2D.UMG_Main|GetBar_MP (Variables|/Script/GAME2D.HUD_All_UI|GetUMG_Main _returnvalue)) (/ NewVal (.ReturnValue (Ability|Attribute|GetFloatAttributefromAbilitySystemComponent (Variables|Default|GetMyASC) "(AttributeName=\"MAX_MP\",Attribute=/Script/GAME2D.BaseAttributeSet:MAX_MP,AttributeOwner=\"/Script/CoreUObject.Class'/Script/GAME2D.BaseAttributeSet'\")")))))))

(event EventArmorChangeEvent事件
  (params (NewVal :type Float%20%28single-precision%29))
  ;[1 1 1] 设置护盾
  (if (> NewVal 0.0)
    (Class|BaseCharacter|ActivateTag (Variables|Default|GetMyASC) "(TagName=\"Player.Equip.HasArmor\")")
    (else
      (Class|BaseCharacter|DeactivateTag (Variables|Default|GetMyASC) "(TagName=\"Player.Equip.HasArmor\")")))
  (Progress|SetPercent (Variables|/Script/GAME2D.UMG_Main|GetBar_Armor (Variables|/Script/GAME2D.HUD_All_UI|GetUMG_Main (Class|MyBlueprintFunctionLibrary|GetHUDAllUI))) (/ NewVal (.ReturnValue (Ability|Attribute|GetFloatAttributefromAbilitySystemComponent (Variables|Default|GetMyASC) "(AttributeName=\"Max_Armor\",Attribute=/Script/GAME2D.BaseAttributeSet:Max_Armor,AttributeOwner=\"/Script/CoreUObject.Class'/Script/GAME2D.BaseAttributeSet'\")")))))

(event EventHPChangeEvent事件
  (params (NewVal :type Float%20%28single-precision%29))
  (bind _returnvalue (Class|MyBlueprintFunctionLibrary|GetHUDAllUI))
  ;[0.01116 1 0 0] 设置血条
  (bind _output_get (Variables|Default|SetNewHP NewVal))
  (Utilities|IsValid _returnvalue
    (:Is%20Valid
      (Progress|SetPercent (Variables|/Script/GAME2D.UMG_Main|GetBar_HP (Variables|/Script/GAME2D.HUD_All_UI|GetUMG_Main _returnvalue)) (/ _output_get (.ReturnValue (Ability|Attribute|GetFloatAttributefromAbilitySystemComponent (Variables|Default|GetMyASC) "(AttributeName=\"MAX_HP\",Attribute=/Script/GAME2D.BaseAttributeSet:MAX_HP,AttributeOwner=\"/Script/CoreUObject.Class'/Script/GAME2D.BaseAttributeSet'\")"))))
      (CallFunction|PlayerDamagePop)
      (if (<= _output_get 0.0)
        (CallFunction|PlayerReturn)))))

(event Input|KeyboardEvents|1
  (params (Key :type Key%20Structure :default "None"))
  ;[0 0.04964 1] 调试板块
  ;;[0 0 0] 检查物品数组
  (:Pressed
    (for _array_element (Variables|/Script/GAME2D.MyGameInstance|GetBackPack_Array (Class|MyBlueprintFunctionLibrary|GetGameInstanceBase))
      (Development|PrintString (Utilities|String|Append (.Name (Utilities|Struct|BreakItem_Struct _array_element)) "     Count:" (Utilities|String|ToString(Integer) (.Count (Utilities|Struct|BreakItem_Struct _array_element))) "    Class:" (Utilities|GetDisplayName (.ItemClass (Utilities|Struct|BreakItem_Struct _array_element))))))))

(event Input|KeyboardEvents|2
  (params (Key :type Key%20Structure :default "None"))
  ;[0 0.04964 1] 调试板块
  (:Pressed
    (bind _asbp_game_instance_base (Utilities|Casting|CastToBP_GameInstanceBase (Class|MyBlueprintFunctionLibrary|GetGameInstanceBase)))
    (for _array_element (Variables|/Script/GAME2D.MyGameInstance|GetEquip_Array _asbp_game_instance_base)
      (Development|PrintString (Utilities|String|Append (.Name (Utilities|Struct|BreakItem_Struct _array_element)) "     Count:" (Utilities|String|ToString(Integer) (.Count (Utilities|Struct|BreakItem_Struct _array_element))) "    Class:" (Utilities|GetDisplayName (.ItemClass (Utilities|Struct|BreakItem_Struct _array_element)))) true true "(R=0.000000,G=0.660000,B=1.000000,A=1.000000)" 2e+01))))

(event Input|KeyboardEvents|5
  (params (Key :type Key%20Structure :default "None"))
  (:Pressed
    (bind _asbp_player_controller (Utilities|Casting|CastToBP_PlayerController (Class|MyBlueprintFunctionLibrary|GetPlayerController)))
    (Default|EventLoadGame _asbp_player_controller)))

(fn ConstructionScript
  (|CallParentFunction))

(fn ActiveAbilitySelf
  (params (AbilityIndex :type Integer))
  (Abilities|TryActivateAbilitiesbyTag (Variables|Default|GetMyASC) (Utilities|Array|Get(acopy) (Variables|Default|GetPlayerAbilityTags) AbilityIndex) true))

(fn JudgeNPC
  (params (HitNPC :type Object%20Object%20Reference))
  (bind _asbase_npc (Utilities|Casting|CastToBaseNPC HitNPC))
  (if (Utilities|Enum|Equal(Enum) (Utilities|String|ToString(Name) (Variables|/Script/GAME2D.BaseNPC|GetNPC_Name _asbase_npc)) (Utilities|String|EnumtoString (Variables|/Script/GAME2D.MyGameInstance|GetTargetNPC (Class|MyBlueprintFunctionLibrary|GetGameInstanceBase))))
    (return true)
    (else
      (return false))))

(fn Interact
  (bind _bp_player (CallFunction|GetPlayerandPC))
  (bind _returnvalue (Transformation|GetActorLocation _bp_player))
  (bind _outhits (Collision|MultiSphereTraceForObjects _returnvalue _returnvalue 3e+01 (Utilities|Array|MakeArray "ObjectTypeQuery3") false (Utilities|Array|MakeArray _bp_player) "None"))
  (if (Utilities|Array|IsNotEmpty _outhits)
    (Utilities|FlowControl|Sequence
      (:then_0
        ;[1 1 1] 与NPC进行交互
        (bind _asbase_npc (Utilities|Casting|CastToBaseNPC (.HitActor (Collision|BreakHitResult (Utilities|Array|Get(acopy) _outhits)))))
        (bind _output_get (Variables|Default|SetHitNPC _asbase_npc))
        (bind _true (CallFunction|JudgeNPC _output_get))
        (if _true
          (Class|TaskSystemComp|SetDialogue (Variables|/Script/GAME2D.BaseNPC|GetTaskSystemComp _asbase_npc))
          (bind _foundwidgets (Widget|GetAllWidgetsOfClass "/Game/System/TaskSystem/BluePrints/UMG_TargetPointer.UMG_TargetPointer_C" true))
          (Utilities|IsValid (Utilities|Array|Get(acopy) _foundwidgets)
            (:Is%20Valid
              (Widget|RemovefromParent (Utilities|Array|Get(acopy) _foundwidgets))))))
      (:then_1
        ;[1 1 1] 与可拾取物进行交互
        (bind _asitem_base (Utilities|Casting|CastToItemBase (.HitActor (Collision|BreakHitResult (Utilities|Array|Get(acopy) _outhits)))))
        (Utilities|IsValid _asitem_base
          (:Is%20Valid
            (bind _output_get_2 (Variables|Default|SetFocusedItem _asitem_base))
            (Class|BackpackComponent|AddItem (Variables|Default|GetBackpackComponent) (Variables|/Script/GAME2D.ItemBase|GetCurrentItemState _output_get_2) _output_get_2))))
      (:then_2
        (bind _asbp_base_box (Utilities|Casting|CastToBP_BaseBox (.HitActor (Collision|BreakHitResult (Utilities|Array|Get(acopy) _outhits)))))
        (Utilities|IsValid _asbp_base_box
          (:Is%20Valid
            (Default|OnActiveBox _asbp_base_box)))))))