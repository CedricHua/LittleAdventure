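; Spawner actor that periodically releases orc enemies at its own location.
; On BeginPlay a looping five-second timer asks the game instance's BaseObjectManager to place an enemy from its object pool there, if that manager is valid.
; An enemy counter increments on each spawn and clears the timer once the limit is reached.
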(event Custom|EventSpawnOrc
  (bind _returnvalue (Class|MyBlueprintFunctionLibrary|GetGameInstanceBase))
  (bind _baseobjectmanager (Variables|/Script/GAME2D.MyGameInstance|GetBaseObjectManager _returnvalue))
  ;[0 0 0] 控制生成
  (Utilities|IsValid _baseobjectmanager
    (:Is%20Valid
      (Class|BaseObjectManager|SetEnemyObjectPool _baseobjectmanager (Transformation|GetActorLocation))
      (bind _result (Math|Integer|IncrementInt (Variables|Default|GetEnemyCount))
        (:%20%20
          (if (== _result 10)
            (Utilities|Time|ClearandInvalidateTimerbyHandle (Variables|Default|GetTimerHandle))))))))

(event EventBeginPlay
  (bind _returnvalue (Utilities|Time|SetTimerbyEvent (delegate Custom|EventSpawnOrc) 5.0 true))
  (Variables|Default|SetTimerHandle _returnvalue))

(fn ConstructionScript)