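; Poisoner enemy character that uses the Gameplay Ability System, extending its parent class.
; BeginPlay grants the GA_Poisoner_Attack ability.
; On HP change, it spawns a damage popout widget and refreshes its cached HP.
; At zero HP, a DoOnce marks it dead, halts movement, awards random experience and game-instance money, then destroys the actor after a short delay.
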(event EventBeginPlay
  (|CallParentFunction)
  (GameplayAbilities|GiveAbility (Variables|Default|GetMyASC) "/Game/GAS/Abilities/Enemy_Abilities/Poisoner/GA_Poisoner_Attack.GA_Poisoner_Attack_C" 0 -1))

(event EventHPChangeEvent事件
  (params (NewVal :type Float%20%28single-precision%29))
  (bind _returnvalue (Class|MyBlueprintFunctionLibrary|GetGameInstanceBase))
  (Utilities|FlowControl|Sequence
    (:then_0
      ;[0 0 0] 判断是否死亡(执行怪物数量加一，判断杀敌数是否够，给玩家加经验)
      (if (<= NewVal 0.0)
        (Utilities|FlowControl|DoOnce false
          (:Completed
            (Variables|Default|SetIsDead? true)
            (Variables|/Script/Engine.CharacterMovementComponent|SetMaxWalkSpeed (Variables|Character|GetCharacterMovement) 0.0)
            (Class|BaseCharacter|GetExperience (Math|Random|RandomFloatinRange 2e+01 3e+01) "/Game/GAS/Abilities/Player_Abilities/GE_LevelUp.GE_LevelUp_C")
            (Variables|/Script/GAME2D.MyGameInstance|SetPlayerMoney _returnvalue (+ (Variables|/Script/GAME2D.MyGameInstance|GetPlayerMoney _returnvalue) (Math|Random|RandomIntegerinRange 10 30)))
            (Utilities|FlowControl|Delay 0.5)
            (Actor|DestroyActor)))))
    (:then_1
      ;[0 0 0] 设置伤害跳字
      (if (!= (Variables|Default|GetCurrentHP) NewVal)
        (bind _returnvalue_2 (UserInterface|CreateWidget "/Game/UMG/DamagePopout.DamagePopout_C" 0 self (- (Variables|Default|GetCurrentHP) NewVal)))
        (UserInterface|Viewport|AddtoViewport _returnvalue_2 0)
        (Variables|Default|SetCurrentHP (.ReturnValue (Ability|Attribute|GetFloatAttributefromAbilitySystemComponent (Variables|Default|GetMyASC) "(AttributeName=\"HP\",Attribute=/Script/GAME2D.BaseAttributeSet:HP,AttributeOwner=\"/Script/CoreUObject.Class'/Script/GAME2D.BaseAttributeSet'\")")))))))

(fn ConstructionScript
  (|CallParentFunction))