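; Orc enemy character built on the Gameplay Ability System, granted GA_OrcAttack on BeginPlay.
; HP changes update the overhead health bar, play a hurt reaction and spawn a damage popup.
; At zero HP it runs a one-time death: counts the kill, stops movement, awards random experience and money, then recycles and destroys itself after a delay.
; OrcAttack calls EnemyState, waits briefly, then calls EnemySpawnAndHit with its ability component.
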(event Custom|OrcAttack
  (CallFunction|EnemyState 0.5)
  (Utilities|FlowControl|Delay 1.0)
  (CallFunction|EnemySpawnandHit (Variables|Default|GetMyASC)))

(event EventBeginPlay
  (|CallParentFunction)
  (GameplayAbilities|GiveAbility (Variables|Default|GetMyASC) "/Game/GAS/Abilities/Enemy_Abilities/ORC/GA_OrcAttack.GA_OrcAttack_C" 0 -1))

(event EventHPChangeEvent事件
  (params (NewVal :type Float%20%28single-precision%29))
  (bind _returnvalue (Class|MyBlueprintFunctionLibrary|GetGameInstanceBase))
  (Utilities|FlowControl|Sequence
    (:then_0
      ;[0 0 0] 更新血条播放受击动画
      (bind _asumg_enemy_hp (Utilities|Casting|CastToUMG_EnemyHP (UserInterface|GetUserWidgetObject (Variables|Default|GetWidget))))
      (Default|SetHPBar _asumg_enemy_hp (/ NewVal (.ReturnValue (Ability|Attribute|GetFloatAttributefromAbilitySystemComponent (Variables|Default|GetMyASC) "(AttributeName=\"MAX_HP\",Attribute=/Script/GAME2D.BaseAttributeSet:MAX_HP,AttributeOwner=\"/Script/CoreUObject.Class'/Script/GAME2D.BaseAttributeSet'\")"))))
      (CallFunction|PlayHurt))
    (:then_1
      ;[0 0 0] 判断是否死亡(执行怪物数量加一，判断杀敌数是否够，给玩家加经验)
      (if (<= NewVal 0.0)
        (Utilities|FlowControl|DoOnce false
          (:Completed
            (bind _asbp_game_instance_base (Utilities|Casting|CastToBP_GameInstanceBase (Game|GetGameInstance)))
            (Default|JudgeCount _asbp_game_instance_base)
            (Variables|Default|SetIsDead? true)
            (Variables|/Script/Engine.CharacterMovementComponent|SetMaxWalkSpeed (Variables|Character|GetCharacterMovement) 0.0)
            (Class|BaseCharacter|GetExperience (Math|Random|RandomFloatinRange 1e+01 2e+01) "/Game/GAS/Abilities/Player_Abilities/GE_LevelUp.GE_LevelUp_C")
            (Variables|/Script/GAME2D.MyGameInstance|SetPlayerMoney _returnvalue (+ (Variables|/Script/GAME2D.MyGameInstance|GetPlayerMoney _returnvalue) (Math|Random|RandomIntegerinRange 10 20)))
            (Utilities|FlowControl|Delay 0.5)
            (Class|BaseEnemy|RecycleSelf)
            (Actor|DestroyActor self)))))
    (:then_2
      ;[0 0 0] 设置伤害跳字
      (if (!= (Variables|Default|GetCurrentHP) NewVal)
        (bind _returnvalue_2 (UserInterface|CreateWidget "/Game/UMG/DamagePopout.DamagePopout_C" 0 self (- (Variables|Default|GetCurrentHP) NewVal)))
        (UserInterface|Viewport|AddtoViewport _returnvalue_2 0)
        (Variables|Default|SetCurrentHP (.ReturnValue (Ability|Attribute|GetFloatAttributefromAbilitySystemComponent (Variables|Default|GetMyASC) "(AttributeName=\"HP\",Attribute=/Script/GAME2D.BaseAttributeSet:HP,AttributeOwner=\"/Script/CoreUObject.Class'/Script/GAME2D.BaseAttributeSet'\")")))))))

(fn ConstructionScript
  (|CallParentFunction))