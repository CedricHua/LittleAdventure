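; AI controller for the Boomer enemy that starts the BT_Boomer behavior tree on BeginPlay.
; Perception updates feed a Hearing function that sets the blackboard bool "Is See Player" true only for a successfully sensed hearing stimulus from an actor tagged Player.
; Any other perception update sets that key false, and despite the key's name no sight check is made.
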(event OnTargetPerceptionUpdated(AIPerception)
  (params (Actor :type Actor%20Object%20Reference) (Stimulus :type AI%20Stimulus%20Structure))
  (CallFunction|Hearing Stimulus Actor))

(event EventBeginPlay
  (AI|RunBehaviorTree "/Game/Characters/Enemy/BluePrints/Enemy_Boomer/BT_Boomer.BT_Boomer"))

(fn ConstructionScript)

(fn Hearing
  (params (AIStimulus :type AI%20Stimulus%20Structure) (Actor :type Actor%20Object%20Reference))
  (bind _returnvalue (Utilities|Name|MakeLiteralName "Is See Player"))
  (bind _returnvalue_2 (AI|GetBlackboard 0))
  (bind _returnvalue_3 (Class|AIPerceptionSystem|GetSenseClassforStimulus AIStimulus))
  (if (Math|Boolean|ANDBoolean (== _returnvalue_3 "/Script/AIModule.AISense_Hearing") (Actor|ActorHasTag Actor "Player") (.bSuccessfullySensed (Utilities|Struct|BreakAIStimulus AIStimulus)))
    (AI|Components|Blackboard|SetValueasBool _returnvalue_2 _returnvalue true)
    (else
      (AI|Components|Blackboard|SetValueasBool _returnvalue_2 _returnvalue false)))
  (return))