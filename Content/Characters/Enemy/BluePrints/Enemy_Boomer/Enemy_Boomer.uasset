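; Boomer enemy Blueprint for an exploding attacker that uses GAS and is granted GA_BoomerAtk at BeginPlay.
; Hearing and range sphere overlaps with the player set Blackboard flags, and Atk sets CanAtk, then destroys the actor after a short delay.
; HP changes spawn damage popups; at zero HP, a one-shot branch updates the kill count, awards random experience and money, then destroys it.
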(event OnComponentBeginOverlap(Sphere_Hearing)
  (params (OverlappedComponent :type Primitive%20Component%20Object%20Reference) (OtherActor :type Actor%20Object%20Reference) (OtherComp :type Primitive%20Component%20Object%20Reference) (OtherBodyIndex :type Integer) (bFromSweep :type Boolean) (SweepResult :type Hit%20Result%20Structure%20%28by%20ref%29))
  (if (== OtherActor (.BP_Player (CallFunction|GetPlayerandPC)))
    (AI|Components|Blackboard|SetValueasBool (AI|GetBlackboard 0) (Utilities|Name|MakeLiteralName "Is See Player") true)))

(event OnComponentBeginOverlap(Sphere1)
  (params (OverlappedComponent :type Primitive%20Component%20Object%20Reference) (OtherActor :type Actor%20Object%20Reference) (OtherComp :type Primitive%20Component%20Object%20Reference) (OtherBodyIndex :type Integer) (bFromSweep :type Boolean) (SweepResult :type Hit%20Result%20Structure%20%28by%20ref%29))
  (if (== OtherActor (.BP_Player (CallFunction|GetPlayerandPC)))
    (AI|Components|Blackboard|SetValueasBool (AI|GetBlackboard 0) (Utilities|Name|MakeLiteralName "Is Player InRange") true)))

(event Custom|Atk
  (Variables|Default|SetCanAtk? true)
  (Utilities|FlowControl|Delay 0.8)
  (Actor|DestroyActor))

(event EventBeginPlay
  (|CallParentFunction)
  (GameplayAbilities|GiveAbility (Variables|Default|GetMyASC) "/Game/GAS/Abilities/Enemy_Abilities/Boomer/GA_BoomerAtk.GA_BoomerAtk_C" 0 -1))

(event Collision|EventActorBeginOverlap
  (params (OtherActor :type Actor%20Object%20Reference))
  ;[1 1 1] 进入爆炸范围执行BoomerAtk
)

(event EventTick
  (params (DeltaSeconds :type Float%20%28single-precision%29))
  (|CallParentFunction DeltaSeconds))

(event EventHPChangeEvent事件
  (params (NewVal :type Float%20%28single-precision%29))
  (bind _returnvalue (Class|MyBlueprintFunctionLibrary|GetGameInstanceBase))
  (Utilities|FlowControl|Sequence
    (:then_0
      ;[0 0 0] 判断是否死亡(执行怪物数量加一，判断杀敌数是否够，给玩家加经验)
      (if (<= NewVal 0.0)
        (Utilities|FlowControl|DoOnce false
          (:Completed
            (bind _asbp_game_instance_base (Utilities|Casting|CastToBP_GameInstanceBase (Game|GetGameInstance)))
            (Default|JudgeCount _asbp_game_instance_base)
            (Variables|Default|SetIsDead? true)
            (Variables|/Script/Engine.CharacterMovementComponent|SetMaxWalkSpeed (Variables|Character|GetCharacterMovement) 0.0)
            (Class|BaseCharacter|GetExperience (Math|Random|RandomFloatinRange 2e+01 3e+01) "/Game/GAS/Abilities/Player_Abilities/GE_LevelUp.GE_LevelUp_C")
            (Variables|/Script/GAME2D.MyGameInstance|SetPlayerMoney _returnvalue (+ (Variables|/Script/GAME2D.MyGameInstance|GetPlayerMoney _returnvalue) (Math|Random|RandomIntegerinRange 20 30)))
            (Utilities|FlowControl|Delay 0.5)
            (Actor|DestroyActor)))))
    (:then_1
      ;[0 0 0] 设置伤害跳字
      (if (!= (Variables|Default|GetCurrentHP) NewVal)
        (bind _returnvalue_2 (UserInterface|CreateWidget "/Game/UMG/DamagePopout.DamagePopout_C" 0 self (- (Variables|Default|GetCurrentHP) NewVal)))
        (UserInterface|Viewport|AddtoViewport _returnvalue_2 0)
        (Variables|Default|SetCurrentHP (.ReturnValue (Ability|Attribute|GetFloatAttributefromAbilitySystemComponent (Variables|Default|GetMyASC) "(AttributeName=\"HP\",Attribute=/Script/GAME2D.BaseAttributeSet:HP,AttributeOwner=\"/Script/CoreUObject.Class'/Script/GAME2D.BaseAttributeSet'\")")))))))

(fn ConstructionScript
  (|CallParentFunction))