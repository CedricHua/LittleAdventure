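; Player controller that handles weapon-equip UI and saving and loading of player progress.
; Equipping Sword or Book records the weapon on the player and swaps the main HUD's attack icon.
; Save packs GAS attributes, location, weapon, and game-instance progression, inventory and mission state into one QuickSave slot.
; Load restores these, re-runs the game instance's Init, rebuilds item arrays, and applies GAS attributes after a fixed delay.
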(event Custom|EventSaveGame
  (bind _bp_player (CallFunction|GetPlayerandPC))
  (bind _myasc (Variables|/Script/GAME2D.BaseCharacter|GetMyASC _bp_player))
  (bind _asbp_game_instance_base (Utilities|Casting|CastToBP_GameInstanceBase (Class|MyBlueprintFunctionLibrary|GetGameInstanceBase)))
  (Class|MySaveGame|QuickSave (Utilities|Struct|MakePlayerSaveData (.ReturnValue (Ability|Attribute|GetFloatAttributefromAbilitySystemComponent _myasc "(AttributeName=\"HP\",Attribute=/Script/GAME2D.BaseAttributeSet:HP,AttributeOwner=\"/Script/CoreUObject.Class'/Script/GAME2D.BaseAttributeSet'\")")) (.ReturnValue (Ability|Attribute|GetFloatAttributefromAbilitySystemComponent _myasc "(AttributeName=\"MP\",Attribute=/Script/GAME2D.BaseAttributeSet:MP,AttributeOwner=\"/Script/CoreUObject.Class'/Script/GAME2D.BaseAttributeSet'\")")) (.ReturnValue (Ability|Attribute|GetFloatAttributefromAbilitySystemComponent _myasc "(AttributeName=\"Armor\",Attribute=/Script/GAME2D.BaseAttributeSet:Armor,AttributeOwner=\"/Script/CoreUObject.Class'/Script/GAME2D.BaseAttributeSet'\")")) (Variables|/Script/GAME2D.MyGameInstance|GetPlayerLevel _asbp_game_instance_base) (Variables|/Script/GAME2D.MyGameInstance|GetPlayerXP _asbp_game_instance_base) (Variables|/Script/GAME2D.MyGameInstance|GetPlayerMoney _asbp_game_instance_base) (Variables|/Script/GAME2D.MyGameInstance|GetBackPack_Array _asbp_game_instance_base) (Variables|/Script/GAME2D.MyGameInstance|GetEquip_Array _asbp_game_instance_base) (Variables|/Script/GAME2D.MyGameInstance|GetMissionIndex _asbp_game_instance_base) (Variables|/Script/GAME2D.MyGameInstance|GetTaskIndex _asbp_game_instance_base) (Variables|/Script/GAME2D.MyGameInstance|GetKillCnt _asbp_game_instance_base) (Variables|/Script/GAME2D.MyGameInstance|GetEquipCnt _asbp_game_instance_base) (Variables|/Script/GAME2D.MyGameInstance|GetTargetNPC _asbp_game_instance_base) (Transformation|GetActorLocation (.BP_Player (CallFunction|GetPlayerandPC))) (Variables|/Game/Characters/Player/Blueprints/BP_Player.BP_Player_C|GetEquippingWeapon (.BP_Player (CallFunction|GetPlayerandPC)))) "GameSave"))

(event Custom|EventLoadGame
  (bind _returnvalue (SaveGame|DoesSaveGameExist "GameSave"))
  (if _returnvalue
    (bind _outsavedata (Class|MySaveGame|QuickLoad "GameSave"))
    (Utilities|FlowControl|Sequence
      (:then_0
        (bind _asbp_game_instance_base (Utilities|Casting|CastToBP_GameInstanceBase (Class|MyBlueprintFunctionLibrary|GetGameInstanceBase)))
        (Variables|/Script/GAME2D.MyGameInstance|SetbShouldCallEvent _asbp_game_instance_base false)
        (Variables|/Script/GAME2D.MyGameInstance|SetPlayerLevel _asbp_game_instance_base (.SaveLevel (Utilities|Struct|BreakPlayerSaveData _outsavedata)))
        (Variables|/Script/GAME2D.MyGameInstance|SetPlayerXP _asbp_game_instance_base (.SaveExp (Utilities|Struct|BreakPlayerSaveData _outsavedata)))
        (Variables|/Script/GAME2D.MyGameInstance|SetPlayerMoney _asbp_game_instance_base (.SaveMoney (Utilities|Struct|BreakPlayerSaveData _outsavedata)))
        (Variables|Default|SetLoadItemArr (.SaveItemArr (Utilities|Struct|BreakPlayerSaveData _outsavedata)))
        (Variables|Default|SetLoadEquipArr (.SaveEquipArr (Utilities|Struct|BreakPlayerSaveData _outsavedata)))
        (Variables|/Script/GAME2D.MyGameInstance|SetMissionIndex _asbp_game_instance_base (.SaveMissionIndex (Utilities|Struct|BreakPlayerSaveData _outsavedata)))
        (Variables|/Script/GAME2D.MyGameInstance|SetKillCnt _asbp_game_instance_base (.SaveKillCnt (Utilities|Struct|BreakPlayerSaveData _outsavedata)))
        (Variables|/Script/GAME2D.MyGameInstance|SetEquipCnt _asbp_game_instance_base (.SaveEquipCnt (Utilities|Struct|BreakPlayerSaveData _outsavedata)))
        (Variables|/Script/GAME2D.MyGameInstance|SetTaskIndex _asbp_game_instance_base (.SaveTaskIndex (Utilities|Struct|BreakPlayerSaveData _outsavedata)))
        (Variables|/Script/GAME2D.MyGameInstance|SetTargetNPC _asbp_game_instance_base (.SaveTargetNPC (Utilities|Struct|BreakPlayerSaveData _outsavedata)))
        (Variables|/Game/Characters/Player/Blueprints/BP_Player.BP_Player_C|SetEquippingWeapon (.BP_Player (CallFunction|GetPlayerandPC)) (.PlayerEquipWeapon (Utilities|Struct|BreakPlayerSaveData _outsavedata)))
        (Transformation|SetActorLocation (.BP_Player (CallFunction|GetPlayerandPC)) (.PlayerLocation (Utilities|Struct|BreakPlayerSaveData _outsavedata)) false false)
        (Class|MyGameInstance|Init (Class|MyBlueprintFunctionLibrary|GetGameInstanceBase))
        (CallFunction|InitEquipArr)
        (CallFunction|InitItemArr))
      (:then_1
        (Utilities|FlowControl|Delay 5.0)
        (Default|LoadGAS (.BP_Player (CallFunction|GetPlayerandPC)) (.SaveHP (Utilities|Struct|BreakPlayerSaveData _outsavedata)) (.SaveMP (Utilities|Struct|BreakPlayerSaveData _outsavedata)) (.SaveArmor (Utilities|Struct|BreakPlayerSaveData _outsavedata)))))))

(event Custom|OnWeaponEquip
  (params (CurrentEquipWeapon :type String))
  (switch string CurrentEquipWeapon
    (:Sword
      (Variables|/Game/Characters/Player/Blueprints/BP_Player.BP_Player_C|SetEquippingWeapon (.BP_Player (CallFunction|GetPlayerandPC)) "Sword")
      (bind _umg_main (Variables|/Script/GAME2D.HUD_All_UI|GetUMG_Main (Class|MyBlueprintFunctionLibrary|GetHUDAllUI))
        (:then
          (Class|UMGMain|ExchangeAtkIcon _umg_main "/Game/UMG/Assets/SwordAttack.SwordAttack"))
        (:else)))
    (:Book
      (Variables|/Game/Characters/Player/Blueprints/BP_Player.BP_Player_C|SetEquippingWeapon (.BP_Player (CallFunction|GetPlayerandPC)) "Book")
      (bind _umg_main_2 (Variables|/Script/GAME2D.HUD_All_UI|GetUMG_Main (Class|MyBlueprintFunctionLibrary|GetHUDAllUI))
        (:then
          (Class|UMGMain|ExchangeAtkIcon _umg_main_2 "/Game/UMG/Assets/BookAttack.BookAttack"))
        (:else)))))

(event Custom|InitItemArr
  (for (_array_element _array_index) (Variables|Default|GetLoadItemArr)
    (bind _asbp_game_instance_base (Utilities|Casting|CastToBP_GameInstanceBase (Class|MyBlueprintFunctionLibrary|GetGameInstanceBase)))
    (Utilities|Array|SetArrayElem (Variables|/Script/GAME2D.MyGameInstance|GetBackPack_Array _asbp_game_instance_base) _array_index (Utilities|Struct|MakeItem_Struct (.ItemClass (Utilities|Struct|BreakItem_Struct _array_element)) (.Name (Utilities|Struct|BreakItem_Struct _array_element)) (.Description (Utilities|Struct|BreakItem_Struct _array_element)) (.Index (Utilities|Struct|BreakItem_Struct _array_element)) (.Icon (Utilities|Struct|BreakItem_Struct _array_element)) (.Count (Utilities|Struct|BreakItem_Struct _array_element)) (.Max_Count (Utilities|Struct|BreakItem_Struct _array_element)) (.Can_Stack (Utilities|Struct|BreakItem_Struct _array_element)) (.EquipIndex (Utilities|Struct|BreakItem_Struct _array_element)) (.Item_Type (Utilities|Struct|BreakItem_Struct _array_element))))))

(event Custom|InitEquipArr
  (for (_array_element _array_index) (Variables|Default|GetLoadEquipArr)
    (bind _asbp_game_instance_base (Utilities|Casting|CastToBP_GameInstanceBase (Class|MyBlueprintFunctionLibrary|GetGameInstanceBase)))
    (Utilities|Array|SetArrayElem (Variables|/Script/GAME2D.MyGameInstance|GetEquip_Array _asbp_game_instance_base) _array_index (Utilities|Struct|MakeItem_Struct (.ItemClass (Utilities|Struct|BreakItem_Struct _array_element)) (.Name (Utilities|Struct|BreakItem_Struct _array_element)) (.Description (Utilities|Struct|BreakItem_Struct _array_element)) (.Index (Utilities|Struct|BreakItem_Struct _array_element)) (.Icon (Utilities|Struct|BreakItem_Struct _array_element)) (.Count (Utilities|Struct|BreakItem_Struct _array_element)) (.Max_Count (Utilities|Struct|BreakItem_Struct _array_element)) (.Can_Stack (Utilities|Struct|BreakItem_Struct _array_element)) (.EquipIndex (Utilities|Struct|BreakItem_Struct _array_element)) (.Item_Type (Utilities|Struct|BreakItem_Struct _array_element))))))

(event EventBeginPlay
  (bind _bp_player (CallFunction|GetPlayerandPC))
  (Utilities|IsValid _bp_player
    (:Is%20Valid
      (Variables|Default|SetBP%20Player _bp_player))))

(fn ConstructionScript)