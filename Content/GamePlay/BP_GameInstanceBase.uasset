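; Base Game Instance that holds player progress, inventory, equipment and task state.
; JudgeCount and JudgeEquip count kills and equips; reaching their thresholds shares one path that advances TaskIndex, runs TaskControl, updates the player's task tip and target, then saves after a short delay.
; InitSelgfVariable resets stats, counters and task target to starting values and restores backpack and equipment arrays from blank templates.
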(event Custom|JudgeCount
  (bind (_bp_player _bp_player_controller) (CallFunction|GetPlayerandPC))
  (bind _result (Math|Integer|IncrementInt (Variables|Default|GetKillCnt))
    (:%20%20
      (Variables|Default|SetKillCnt _result)
      (if (== _result 20)
        (bind _result_2 (Math|Integer|IncrementInt (Variables|Default|GetTaskIndex))
          (:%20%20
            (Variables|Default|SetTaskIndex _result_2)
            (Class|MyGameInstance|TaskControl)
            (Class|TaskSystemComp|SetTaskTipandTarget (Variables|/Script/GAME2D.BaseCharacter|GetTaskSystemComp _bp_player))
            (Utilities|FlowControl|Delay 2.0)
            (Default|EventSaveGame _bp_player_controller)))))))

(event Custom|JudgeEquip
  (bind (_bp_player _bp_player_controller) (CallFunction|GetPlayerandPC))
  (bind _result (Math|Integer|IncrementInt (Variables|Default|GetEquipCnt))
    (:%20%20
      (bind _output_get (Variables|Default|SetEquipCnt _result))
      (if (== _output_get 2)
        (bind _result_2 (Math|Integer|IncrementInt (Variables|Default|GetTaskIndex))
          (:%20%20
            (Variables|Default|SetTaskIndex _result_2)
            (Class|MyGameInstance|TaskControl)
            (Class|TaskSystemComp|SetTaskTipandTarget (Variables|/Script/GAME2D.BaseCharacter|GetTaskSystemComp _bp_player))
            (Utilities|FlowControl|Delay 2.0)
            (Default|EventSaveGame _bp_player_controller)))))))

(event Custom|InitSelgfVariable
  (Utilities|FlowControl|Sequence
    (:then_0
      (Variables|Default|SetPlayerLevel 0)
      (Variables|Default|SetPlayerXP 0.0)
      (Variables|Default|SetPlayerMoney 0)
      (Variables|Default|SetMissionIndex 0)
      (Variables|Default|SetTaskIndex 1)
      (Variables|Default|SetTargetNPC "Ewan")
      (Variables|Default|SetKillCnt 0)
      (Variables|Default|SetEquipCnt 0)
      (Variables|Default|SetbShouldCallEvent true))
    (:then_1
      (Variables|Default|SetBackPack_Array (Variables|Default|GetBlankBPArr))
      (Variables|Default|SetEquip_Array (Variables|Default|GetBlankEquipArr)))))