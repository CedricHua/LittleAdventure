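; Player Gameplay Ability for the book attack, which fires a flipbook projectile in the player's movement direction.
; On activation it commits, then sets a player state with a brief delay and reduced walk speed.
; It requests the projectile from the game instance's object manager pool, offset from the player and driven by the player's velocity values.
; The graph never calls EndAbility, and its OnEndAbility event is unused.
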(event Ability|EventActivateAbility
  (bind _bp_player (CallFunction|GetPlayerandPC))
  (Ability|CommitAbility)
  (Default|SetPlayerState (.BP_Player (CallFunction|GetPlayerandPC)) 0.5 1e+01)
  (Variables|Default|SetGameInstanceBase (Class|MyBlueprintFunctionLibrary|GetGameInstanceBase))
  (Class|BaseObjectManager|SetObjectPool (Variables|/Script/GAME2D.MyGameInstance|GetBaseObjectManager (Variables|Default|GetGameInstanceBase)) (+ (Transformation|GetActorLocation _bp_player) "20.000000,0.000000,0.000000") (Math|Vector|MakeVector (* (Variables|/Script/GAME2D.BaseCharacter|GetVel_X _bp_player) 3.5e+02) (* (Variables|/Script/GAME2D.BaseCharacter|GetVel_Y _bp_player) 3.5e+02) 0.0) "/Game/FX/Animation/RocketFire1.RocketFire1" 1.0))

(event Ability|EventOnEndAbility
  (params (bWasCancelled :type Boolean)))